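; Base player character that moves, looks and fires projectiles from the camera, with limited lives and ammo.
; On BeginPlay it reads default lives and ammo from UserGameMode, creates the UI widget and stores its start location for teleport resets.
; Running out of lives or firing the last projectile triggers PlayerFail.
; PlayerFail and PlayerWin show their screens, then restore counters and reset the widget's timer and displays, without teleporting the player.
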(event `CustomEvent`)

(event `self.ReceiveBeginPlay`
  (`self.SetDefaultLivesF`)
  (`self.SetDefaultProjectilesNumberF`)
  (`self.AddWidgetUIF`)
  (`self.SetDefaultLocation`))

(event `InputAxis|MousePitch`
  (params (AxisValue :type "Float (single-precision)"))
  (`self.AddControllerPitchInput` AxisValue))

(event `InputAxis|MouseYaw`
  (params (AxisValue :type "Float (single-precision)"))
  (`self.AddControllerYawInput` AxisValue))

(event `PlayerFail`
  (`/Game/Blueprints/Widgets/UserInterfaceW.ShowHideFailScreenF` (`self.WidgetRef`) true)
  (`self.RestartGameF`))

(event `InputAxis|MoveForward`
  (params (AxisValue :type "Float (single-precision)"))
  (`self.AddMovementInput` (`KismetMathLibrary.GetForwardVector` (`self.K2_GetActorRotation`)) AxisValue))

(event `PlayerWin`
  (`/Game/Blueprints/Widgets/UserInterfaceW.ShowHideWonScreenF` (`self.WidgetRef`) true)
  (`self.RestartGameF`))

(event `InputAction|Fire`
  (params (Key :type "Key Structure"))
  (:`Pressed`
    (`self.FireF`)))

(event `InputAxis|MoveRight`
  (params (AxisValue :type "Float (single-precision)"))
  (`self.AddMovementInput` (`KismetMathLibrary.GetRightVector` (`self.K2_GetActorRotation`)) AxisValue))

(event `Trap`)

(fn `AddWidgetUIF`
  (bind _returnvalue (`|CreateWidget` "/Game/Blueprints/Widgets/UserInterfaceW.UserInterfaceW_C"))
  (bind _output_get (set `self.WidgetRef` _returnvalue))
  (`UserWidget.AddToViewport` _output_get 0))

(fn `FireF`
  (bind _camera (`self.Camera`))
  (bind _returnvalue (`SceneComponent.K2_GetComponentRotation` _camera))
  (`self.ReduceProjectilesNumber`)
  (`|SpawnActorFromClass` "/Game/Blueprints/Projectile/ProjectileBP.ProjectileBP_C" (`KismetMathLibrary.MakeTransform` (+ (`SceneComponent.K2_GetComponentLocation` _camera) (* (`KismetMathLibrary.GetForwardVector` _returnvalue) 100.0)) _returnvalue) "AlwaysSpawn" "OverrideRootScale" null null))

(fn `ReducePlayerLivesF`
  (if (< (`self.Lives`) 1)
    (`self.PlayerFail`)
    (else
      (set `self.Lives` (- (`self.Lives`) 1))
      (`/Game/Blueprints/Widgets/UserInterfaceW.SetDefaultLivesF` (`self.WidgetRef`)))))

(fn `ReduceProjectilesNumber`
  (bind _projectilesnumber (`self.ProjectilesNumber`))
  (if (< _projectilesnumber 2)
    (`self.PlayerFail`)
    (else
      (set `self.ProjectilesNumber` (- _projectilesnumber 1))
      (`/Game/Blueprints/Widgets/UserInterfaceW.SetDefaultProjectilesNumber` (`self.WidgetRef`)))))

(fn `ResetPlayerValuesF`
  (`self.TeleportToStartF`))

(fn `RestartGameF`
  (bind _widgetref (`self.WidgetRef`))
  (`self.SetDefaultProjectilesNumberF`)
  (`self.SetDefaultLivesF`)
  (`/Game/Blueprints/Widgets/UserInterfaceW.FocusPlayerControlerOnUIorGame` _widgetref true)
  (`/Game/Blueprints/Widgets/UserInterfaceW.SetDefaultLivesF` _widgetref)
  (`/Game/Blueprints/Widgets/UserInterfaceW.SetDefaultTime` _widgetref)
  (`/Game/Blueprints/Widgets/UserInterfaceW.ClearTimerF` _widgetref)
  (`/Game/Blueprints/Widgets/UserInterfaceW.SetDefaultProjectilesNumber` _widgetref))

(fn `SetDefaultLivesF`
  (bind _asuser_game_mode (cast `/Game/Blueprints/SuperClasses/UserGameMode` (`GameplayStatics.GetGameMode`)))
  (set `self.Lives` (`/Game/Blueprints/SuperClasses/UserGameMode.DefaultLivesGiveToPlayer` _asuser_game_mode)))

(fn `SetDefaultLocation`
  (set `self.PlayerLocation` (`self.K2_GetActorLocation`)))

(fn `SetDefaultProjectilesNumberF`
  (bind _asuser_game_mode (cast `/Game/Blueprints/SuperClasses/UserGameMode` (`GameplayStatics.GetGameMode`)))
  (set `self.ProjectilesNumber` (`/Game/Blueprints/SuperClasses/UserGameMode.DefaultProjectilesNumberGivenToPlayer` _asuser_game_mode)))

(fn `TeleportToStartF`
  (`self.K2_SetActorRelativeLocation` (`self.PlayerLocation`)))

(fn `UserConstructionScript`)